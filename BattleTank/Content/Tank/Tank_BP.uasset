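; Player tank Blueprint that handles driving, turret aiming, firing and camera switching.
; BeginPlay initialises the TankAiming component with barrel and turret, TankMovement with both tracks, and hands itself to the health bar widget.
; Input feeds movement intents and fire to those components, rotates the azimuth gimbal and spring arm to aim, and toggles first- and third-person cameras.
; Tick scales damage smoke size inversely with health percent.
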(event `self.ReceiveBeginPlay`
  (`TankAimingComponent.Initialise` (`self.TankAiming`) (`self.TankBarrel`) (`self.TankTurret`))
  (`TankMovementComponent.Initialise` (`self.TankMovement`) (`self.LeftTrack`) (`self.RightTrack`))
  (`self.InitialiseHealthBar`))

(event `self.ReceiveTick`
  (params (DeltaSeconds :type "Float (single-precision)"))
  (`ParticleSystemComponent.SetVectorParameter` (`self.DamageSmoke`) "size" (`KismetMathLibrary.Conv_DoubleToVector` (* (/ 1.0 (+ (`self.GetHealthPercent`) 0.001)) 100.0))))

(event `InputAxis|MoveForwards`
  (params (AxisValue :type "Float (single-precision)"))
  ;[1 1 1] Movement Input Binding
  (`TankMovementComponent.IntendMoveForward` (`self.TankMovement`) AxisValue))

(event `InputAxis|AimAzimuth`
  (params (AxisValue :type "Float (single-precision)"))
  ;[1 1 1] Crosshair Movement
  (`SceneComponent.K2_AddLocalRotation` (`self.AzimuthGimbal`) (`KismetMathLibrary.MakeRotator` 0.0 0.0 AxisValue) false false))

(event `InputAxis|TurnRight`
  (params (AxisValue :type "Float (single-precision)"))
  ;[1 1 1] Movement Input Binding
  (`TankMovementComponent.IntendTurnRight` (`self.TankMovement`) AxisValue))

(event `InputAxis|AimElevation`
  (params (AxisValue :type "Float (single-precision)"))
  ;[1 1 1] Crosshair Movement
  (`SceneComponent.K2_AddLocalRotation` (`self.SpringArm`) (`KismetMathLibrary.MakeRotator` 0.0 AxisValue) false false))

(event `InputAction|SwapCam`
  (params (Key :type "Key Structure"))
  (:`Pressed`
    (`ActorComponent.ToggleActive` (`self.1st Person`))
    (`ActorComponent.ToggleActive` (`self.3rd Person`))))

(event `InputAction|Fire`
  (params (Key :type "Key Structure"))
  ;[1 1 1] Crosshair Movement
  (:`Pressed`
    (`TankAimingComponent.Fire` (`self.TankAiming`))))

(fn `InitialiseHealthBar`
  (bind _ashealthbar_bp (cast `/Game/UI/Healthbar_BP` (`WidgetComponent.GetUserWidgetObject` (`self.Widget`))))
  (set `/Game/UI/Healthbar_BP.TankRef` self _ashealthbar_bp))

(fn `UserConstructionScript`)